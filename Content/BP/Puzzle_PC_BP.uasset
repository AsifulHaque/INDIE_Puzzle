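; Touch player controller for a Rubik's cube puzzle, where the pawn walks on cube surfaces and swipes rotate the cube.
; A tap checks the touched surface against paths from the standing RubicsCubeUnit, then a timeline moves the pawn there and attaches it.
; A swipe rotates a slice found by box overlap from hit normal and direction, or the whole cube without a target unit.
; A one-second delay locks input during rotation.
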(event EventBeginPlay
  ;[1 1 1] BEGINPLAY
  (Variables|Default|SetbShowMouseCursor true)
  (CallFunction|InitializePlacement))

(event Input|ActionEvents|InputActionPauseMenu
  (params (Key :type Key%20Structure :default "None"))
  ;[1 1 1] Call Pause menu
  (:Pressed
    (bind _asgameplay_gm_bp (Utilities|Casting|CastToGameplayGM_BP (Game|GetGameMode)))
    (Default|PauseMenu _asgameplay_gm_bp)))

(event Input|TouchEvents|InputTouch
  (params (Location :type Vector) (FingerIndex :type ETouchIndex%20Enum))
  (bind _targetloc (Variables|PlayerMovement|GetTargetLoc))
  ;[1 1 1] Main Gameplay Control
  (:Pressed
    (Variables|PlayerMovement|SetTouchStartLoc Location)
    (if (and (not (Variables|PlayerMovement|GetisMoving)) (not (Variables|CubeRotation|GetCubeRotating)))
      (CallFunction|UpdateAvailablePaths)
      (bind _hit_ (CallFunction|SetTargetLocRot))
      (Variables|PlayerMovement|SetCanMove (and _hit_ (not (Variables|CubeRotation|GetCubeRotating))))))
  (:Released
    (if (Math|Boolean|ANDBoolean (Variables|PlayerMovement|GetCanMove) (not (Variables|PlayerMovement|GetisMoving)) (not (Variables|CubeRotation|GetCubeRotating)))
      (Variables|PlayerMovement|SetisMoving true)
      (bind _returnvalue (Rendering|Decal|SpawnDecalatLocation "/Game/MobileStarterContent/Materials/M_Cursor_Decal_Inst.M_Cursor_Decal_Inst" "32.000000,32.000000,32.000000" _targetloc (Math|Conversions|RotationFromXVector _targetloc) 0.0))
      (Rendering|Components|Decal|SetFadeOut _returnvalue 0.0 1.0 true)
      (Transformation|DetachFromActor (Game|Player|GetPlayerPawn 0) "KeepWorld" "KeepWorld" "KeepWorld")
      (Variables|Default|SetPrevTransform (Transformation|GetActorTransform (Game|Player|GetPlayerPawn 0)))
      (Variables|PlayerMovement|SetCanMove false)
      (Utilities|Array|Clear (Variables|PlayerMovement|GetAvailablePaths))
      (bind _movelerp (Timeline|Movement PlayFromStart)
        (:Update
          (Transformation|SetActorTransform (Game|Player|GetPlayerPawn 0) (Math|Transform|MakeTransform (Math|Vector|Lerp(Vector) (.location (Variables|Default|GetPrevTransform)) (Variables|PlayerMovement|GetTargetLoc) _movelerp) (Math|Rotator|Lerp(Rotator) (.rotation (Variables|Default|GetPrevTransform)) (Variables|PlayerMovement|GetTargetRot) _movelerp true) "1,1,1")))
        (:Finished
          ;;[1 1 1] Attach to the cube
          (Transformation|AttachActorToActor (Game|Player|GetPlayerPawn 0) (Variables|PlayerMovement|GetTargetCubeActor) "None" "KeepWorld" "KeepWorld" "KeepWorld" true)
          (Variables|PlayerMovement|SetisMoving false)))))
  (:Moved
    (if (not (Variables|CubeRotation|GetCubeRotating))
      (bind _shouldrotate_ (CallFunction|DetectLiteralSwipe Location))
      (if _shouldrotate_
        (CallFunction|GetCubestoRotate)
        ;;[1 1 1] CubeRotationDuration
        (Variables|CubeRotation|SetCubeRotating true)
        (Utilities|FlowControl|Delay 1.0)
        (Variables|CubeRotation|SetCubeRotating false)))))

(fn ConstructionScript)

(fn SetTargetLocRot
  (bind _surfaceobjecttype (Variables|PlayerMovement|GetSurfaceObjectType))
  (bind _hitresult (Class|PlayerController|GetHitResultUnderFingerforObjects "Touch1" _surfaceobjecttype true))
  (bind (_bblockinghit _binitialoverlap _time _distance _location _impactpoint _normal _impactnormal _physmat _hitactor _hitcomponent) (Collision|BreakHitResult _hitresult))
  (if _bblockinghit
    (bind _asrubics_cube_unit (Utilities|Casting|CastToRubicsCubeUnit _hitactor)
      (:then
        ;[1 1 1] Used For Rotating Cubes
        (Variables|PlayerMovement|SetTargetCubeActor _asrubics_cube_unit)
        (Variables|Default|SetTargetSurface _hitcomponent)
        (Variables|Default|SetImpactNormal _impactnormal)
        (Variables|Default|SetImpactPoint _impactpoint)
        (LocalVariables|SetOutputMoveOk? false)
        ;[1 1 1] Detect : Clicked Surface == Available Path
        (bind _array_element (Utilities|Array|ForEachLoopwithBreak (Variables|PlayerMovement|GetAvailablePaths) :!label _label)
          (:LoopBody
            (if (== _array_element _hitcomponent)
              (Variables|PlayerMovement|SetTargetLoc (Transformation|GetWorldLocation _hitcomponent))
              (Variables|PlayerMovement|SetTargetRot (Transformation|GetWorldRotation _hitcomponent))
              (LocalVariables|SetOutputMoveOk? true)
              (goto _label Break)))
          (:Completed
            (return (LocalVariables|GetOutputMoveOk?)))))
      (:CastFailed
        (Variables|PlayerMovement|SetTargetCubeActor 0 :!label _label_2)
        (return false)))
    (else
      (goto _label_2))))

(fn UpdateAvailablePaths
  (bind _returnvalue (Game|Player|GetPlayerPawn 0))
  (bind _returnvalue_2 (Transformation|GetActorLocation _returnvalue))
  (bind _outhit (Collision|LineTraceForObjects _returnvalue_2 (+ _returnvalue_2 (* (Transformation|GetActorUpVector _returnvalue) -1e+01)) (Variables|PlayerMovement|GetSurfaceObjectType) false 0 "None"))
  (bind _asrubics_cube_unit (Utilities|Casting|CastToRubicsCubeUnit (.HitActor (Collision|BreakHitResult _outhit))))
  (if (Components|ComponentHasTag (.HitComponent (Collision|BreakHitResult _outhit)) "Walkable")
    (Default|CalcNav _asrubics_cube_unit (.HitComponent (Collision|BreakHitResult _outhit)))
    (Utilities|Array|Clear (Variables|PlayerMovement|GetAvailablePaths))
    (Variables|PlayerMovement|SetAvailablePaths (Variables|/Game/BP/RubicsCubeUnit.RubicsCubeUnit_C|GetAvailablePathComp _asrubics_cube_unit))))

(fn DetectAnglularSwipeDir
  (params (CurrentTouchLoc :type Vector))
  (bind _touchstartloc (Variables|PlayerMovement|GetTouchStartLoc))
  (bind _returnvalue (- _touchstartloc CurrentTouchLoc))
  (if (> (Math|Vector|VectorLength (- _touchstartloc CurrentTouchLoc)) 1e+01)
    (if (and (< (.x _returnvalue) 0.0) (> (.y _returnvalue) 0.0))
      (Variables|CubeRotation|SetSwipType "NewEnumerator0")
      ;[1 1 1] TODO Remove Debug
      (return true)
      (elif (and (< (.x _returnvalue) 0.0) (< (.y _returnvalue) 0.0))
        (Variables|CubeRotation|SetSwipType "NewEnumerator2")
        (return true)
        (elif (and (> (.x _returnvalue) 0.0) (> (.y _returnvalue) 0.0))
          (Variables|CubeRotation|SetSwipType "NewEnumerator1")
          (return true)
          (elif (and (> (.x _returnvalue) 0.0) (< (.y _returnvalue) 0.0))
            (Variables|CubeRotation|SetSwipType "NewEnumerator3")
            (return true)))))
    (else
      (return false))))

(fn GetCubestoRotate
  (bind _impactnormal (Variables|Default|GetImpactNormal))
  (bind _targetsurface (Variables|Default|GetTargetSurface))
  (bind _returnvalue (Transformation|GetWorldLocation _targetsurface))
  (Utilities|IsValid (Variables|PlayerMovement|GetTargetCubeActor)
    (:Is%20Valid
      (if (== (.x _impactnormal) -1.0)
        (bind _outactors (Collision|BoxOverlapActors _returnvalue (Utilities|Select :Index (Variables|CubeRotation|GetLitSwipDir) :NewEnumerator0 "300.000000,300.000000,10.000000" :NewEnumerator1 "300.000000,300.000000,10.000000" :NewEnumerator2 "300.000000,10.000000,300.000000" :NewEnumerator3 "300.000000,10.000000,300.000000") (Utilities|Array|MakeArray "ObjectTypeQuery2") "/Game/BP/RubicsCubeUnit.RubicsCubeUnit_C" :!class /Script/Engine.KismetSystemLibrary :!label _label))
        (for _array_element _outactors
          (Class|RotationInterface|Rotate(Message) _array_element (Utilities|Select :Index (Variables|CubeRotation|GetLitSwipDir) :NewEnumerator0 "0,90.000000, 0" :NewEnumerator1 "0.000000,-90.000000,0.000000" :NewEnumerator2 "-90.000000, 0,0.000000" :NewEnumerator3 "90.000000, 0,0.000000")))
        (elif (== (.y _impactnormal) -1.0)
          ;[1 1 1] Debug
          (bind _outactors_2 (Collision|BoxOverlapActors _returnvalue (Utilities|Select :Index (Variables|CubeRotation|GetLitSwipDir) :NewEnumerator0 "300.000000,300.000000,10.000000" :NewEnumerator1 "300.000000,300.000000,10.000000" :NewEnumerator2 "10.000000,300.000000,300.000000" :NewEnumerator3 "10.000000,300.000000,300.000000") (Utilities|Array|MakeArray "ObjectTypeQuery2") "/Game/BP/RubicsCubeUnit.RubicsCubeUnit_C" :!class /Script/Engine.KismetSystemLibrary))
          (for _array_element_2 _outactors_2
            (Class|RotationInterface|Rotate(Message) _array_element_2 (Utilities|Select :Index (Variables|CubeRotation|GetLitSwipDir) :NewEnumerator0 "0,90.000000, 0" :NewEnumerator1 "0.000000,-90.000000,0.000000" :NewEnumerator2 "0.000000, 0,90.000000" :NewEnumerator3 "0.000000, 0,-90.000000")))
          (elif (== (.z _impactnormal) 1.0)
            (bind _outactors_3 (Collision|BoxOverlapActors _returnvalue (Utilities|Select :Index (Variables|CubeRotation|GetLitSwipDir) :NewEnumerator0 "300.000000,10.000000,300.000000" :NewEnumerator1 "300.000000,10.000000,300.000000" :NewEnumerator2 "10.000000,300.000000,300.000000" :NewEnumerator3 "10.000000,300.000000,300.000000") (Utilities|Array|MakeArray "ObjectTypeQuery2") "/Game/BP/RubicsCubeUnit.RubicsCubeUnit_C" :!class /Script/Engine.KismetSystemLibrary))
            (for _array_element_3 _outactors_3
              (Class|RotationInterface|Rotate(Message) _array_element_3 (Utilities|Select :Index (Variables|CubeRotation|GetLitSwipDir) :NewEnumerator0 "-90.000000,0.000000,0.000000" :NewEnumerator1 "90.000000,0.000000,0.000000" :NewEnumerator2 "0.000000,0.000000,90.000000" :NewEnumerator3 "0.000000,0.000000,-90.000000")))
            (else
              (goto _label))))))
    (:Is%20Not%20Valid
      ;[1 1 1] Rotate Whole Cube
      (bind _outactors_4 (Actor|GetAllActorsOfClass "/Game/BP/RubicsCubeUnit.RubicsCubeUnit_C"))
      (for _array_element_4 _outactors_4
        (Class|RotationInterface|Rotate(Message) _array_element_4 (Utilities|Select :Index (Variables|CubeRotation|GetLitSwipDir) :NewEnumerator0 "0,90.000000, 0" :NewEnumerator1 "0.000000,-90.000000,0.000000" :NewEnumerator2 "-90.000000, 0,0.000000" :NewEnumerator3 "90.000000, 0,0.000000"))))))

(fn InitializePlacement
  (bind _returnvalue (Game|Player|GetPlayerPawn 0))
  (bind _returnvalue_2 (Game|Player|GetPlayerPawn 0))
  (bind _returnvalue_3 (Transformation|GetActorLocation _returnvalue_2))
  (bind _outhit (Collision|LineTraceForObjects _returnvalue_3 (+ _returnvalue_3 (* (Transformation|GetActorUpVector _returnvalue_2) -1e+01)) (Variables|PlayerMovement|GetSurfaceObjectType) false 0 "None"))
  (Utilities|Casting|CastToRubicsCubeUnit (.HitActor (Collision|BreakHitResult _outhit)))
  (if (Components|ComponentHasTag (.HitComponent (Collision|BreakHitResult _outhit)) "Walkable")
    (Transformation|SetActorTransform _returnvalue (Math|Transform|MakeTransform (.Location (Math|Transform|BreakTransform (Transformation|GetWorldTransform (.HitComponent (Collision|BreakHitResult _outhit))))) (.Rotation (Math|Transform|BreakTransform (Transformation|GetWorldTransform (.HitComponent (Collision|BreakHitResult _outhit))))) "1,1,1"))
    (Transformation|AttachActorToActor _returnvalue (.HitActor (Collision|BreakHitResult _outhit)) "None" "KeepWorld" "KeepWorld" "KeepWorld" true)))

(fn DetectLiteralSwipe
  (params (CurrentTouchLoc :type Vector))
  (bind _touchstartloc (Variables|PlayerMovement|GetTouchStartLoc))
  (bind _returnvalue (- _touchstartloc CurrentTouchLoc))
  (if (> (Math|Vector|VectorLength (- _touchstartloc CurrentTouchLoc)) 1e+01)
    (if (> (Math|Float|Absolute(Float) (.x _returnvalue)) (Math|Float|Absolute(Float) (.y _returnvalue)))
      (if (< (.x _returnvalue) 0.0)
        (Variables|CubeRotation|SetLitSwipDir "NewEnumerator1")
        (else
          (Variables|CubeRotation|SetLitSwipDir "NewEnumerator0")))
      (elif (< (.y _returnvalue) 0.0)
        (Variables|CubeRotation|SetLitSwipDir "NewEnumerator3")
        (else
          (Variables|CubeRotation|SetLitSwipDir "NewEnumerator2"))))
    (return true)
    (else
      (return false))))