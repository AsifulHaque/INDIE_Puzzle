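; CubeUnit_BP is a cube unit that finds the walkable cubes next to it, apparently for grid navigation.
; NavSearch clears AvailableCubes, then refills it from the overlaps of four NavDetector components.
; AddOverlapingCubes keeps other CubeUnit_BP actors flagged Walkable, without checking for duplicates.
; NavSearch also prints each resulting cube's name as debug output.
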(fn ConstructionScript)

(fn NavSearch
  (Utilities|Array|Clear (Variables|Default|GetAvailableCubes))
  (CallFunction|AddOverlapingCubes (Variables|Default|GetNavDetector01))
  (CallFunction|AddOverlapingCubes (Variables|Default|GetNavDetector02))
  (CallFunction|AddOverlapingCubes (Variables|Default|GetNavDetector03))
  (CallFunction|AddOverlapingCubes (Variables|Default|GetNavDetector04))
  ;[1 1 1] Debug
  (for _array_element (Variables|Default|GetAvailableCubes)
    (Development|PrintString (Utilities|GetObjectName _array_element))))

(fn AddOverlapingCubes
  (params (Detector :type Primitive%20Component%20Object%20Reference))
  (for _array_element (Collision|GetOverlappingActors Detector "CubeUnit_BP_C" :!class /Script/Engine.PrimitiveComponent)
    (if (!= _array_element self)
      (bind _ascube_unit_bp (Utilities|Casting|CastToCubeUnit_BP _array_element))
      (if (Variables|CubeUnit_BP_C|GetWalkable? _ascube_unit_bp)
        (Utilities|Array|Add (Variables|Default|GetAvailableCubes) _ascube_unit_bp)))))