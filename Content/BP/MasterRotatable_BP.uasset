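; Base Blueprint for rotatable actors that turn in animated quarter-turn steps.
; The Rotate event takes a clockwise flag and saves the starting rotation, then a timeline lerps the actor along the shortest path to that rotation combined with a 90-degree offset in the chosen direction.
; A CanRotate gate ignores further calls until the timeline finishes.
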(event Custom|Rotate
  (params (ClockWise? :type Boolean))
  ;[1 1 1] Rotate
  (if (Variables|Default|GetCanRotate?)
    (Variables|Default|SetCanRotate? false)
    (Variables|Default|SetStartRotation (Transformation|GetActorRotation))
    (bind _rtrack (Timeline|RotationTL PlayFromStart)
      (:Update
        (Transformation|SetActorRotation (Math|Rotator|Lerp(Rotator) (Variables|Default|GetStartRotation) (Math|Rotator|CombineRotators (Variables|Default|GetStartRotation) (select ClockWise? "0.000000, 0,90.000000" "0.000000, 0,-90.000000")) _rtrack true)))
      (:Finished
        (Variables|Default|SetCanRotate? true)))))

(fn ConstructionScript)