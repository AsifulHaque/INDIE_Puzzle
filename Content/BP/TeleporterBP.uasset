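; Teleporter actor that moves the player pawn to a destination when it overlaps the actor.
; After a one-second delay, it snaps the pawn to TargetActor's location and rotation, or to TargetLocation if no valid actor is set.
; When SwitchCamera is on and TargetCamera is valid, it then blends the player's view to that camera.
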(event Collision|EventActorBeginOverlap
  (params (OtherActor :type Actor%20Object%20Reference))
  (bind _returnvalue (Game|Player|GetPlayerPawn 0))
  (bind _targetactor (Variables|Teleport|GetTargetActor))
  ;[1 1 1] Teleport at overlap
  (if (== OtherActor (Game|Player|GetPlayerPawn 0))
    (Utilities|FlowControl|Delay 1.0)
    (Utilities|IsValid (Variables|Teleport|GetTargetActor)
      (:Is%20Valid
        (Transformation|SetActorTransform _returnvalue (Math|Transform|MakeTransform (Transformation|GetActorLocation _targetactor) (Transformation|GetActorRotation _targetactor) "1,1,1")))
      (:Is%20Not%20Valid
        (Transformation|SetActorLocation _returnvalue (Variables|Teleport|GetTargetLocation) false true)))
    (if (and (Variables|Teleport|GetSwitchCamera?) (Utilities|IsValid (Variables|Teleport|GetTargetCamera)))
      (Game|Player|SetViewTargetwithBlend (Game|GetPlayerController 0) (Variables|Teleport|GetTargetCamera) 1.0 "VTBlend_Cubic" 0.0 false))))

(fn ConstructionScript)