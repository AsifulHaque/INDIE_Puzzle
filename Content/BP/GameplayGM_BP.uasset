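; GameplayGM_BP is the gameplay game mode Blueprint that handles level progression and opens the level-complete and pause menu screens.
; OpenNextLevel finds the current level in the LevelNames array and opens the following entry, wrapping from the last back to the first.
; LevelComplete and PauseMenu each create their widget for the first player controller and add it to the viewport, without changing pause state or input mode.
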(fn ConstructionScript)

(fn OpenNextLevel
  (bind _levelnames (Variables|Levels|GetLevelNames))
  (bind _returnvalue (Game|GetCurrentLevelName true))
  (for (_array_element _array_index) _levelnames
    (if (Utilities|Enum|Equal(Enum) _returnvalue (Utilities|String|ToString(Name) _array_element))
      (Game|OpenLevel(byName) (Utilities|Array|Get(acopy) _levelnames (select (== (+ _array_index 1) (Utilities|Array|Length _levelnames)) 0 (+ _array_index 1)))))))

(fn LevelComplete
  (bind _returnvalue (UserInterface|CreateWidget "/Game/Widgets/CompleteLevelW.CompleteLevelW_C" (Game|GetPlayerController 0)))
  (UserInterface|Viewport|AddtoViewport _returnvalue 0))

(fn PauseMenu
  (bind _returnvalue (UserInterface|CreateWidget "/Game/Widgets/PauseMenuW.PauseMenuW_C" (Game|GetPlayerController 0)))
  (UserInterface|Viewport|AddtoViewport _returnvalue 0))